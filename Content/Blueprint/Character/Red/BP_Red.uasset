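; BP_Red is the playable top-down 2D character, which creates the main HUD and adds its input mapping on BeginPlay.
; Move input drives movement and swaps four-direction walk flipbooks through UpdateAnimation, which also holds the idle flipbook logic for input release.
; Interact scans actors overlapping InteractCheck, showing a BP_PickUp's item or a BP_Green's dialogue on the HUD.
; A retriggerable delay then hides the message box.
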(event `self.ReceiveBeginPlay`
  (bind _returnvalue (`GameplayStatics.GetPlayerController` 0))
  (`|ExecutionSequence`
    (:`then_0`
      (bind _returnvalue_2 (`|CreateWidget` "/Game/Widgets/WBP_MainHUD.WBP_MainHUD_C"))
      (`UserWidget.AddToViewport` _returnvalue_2 0)
      (set `self.MainHUD` _returnvalue_2))
    (:`then_1`
      (if (`KismetSystemLibrary.IsValid` _returnvalue)
        (`EnhancedInputSubsystemInterface.AddMappingContext` (pcsubsystem `EnhancedInputLocalPlayerSubsystem` _returnvalue) "/Game/Inputs/IMC_TopDown.IMC_TopDown" 0 (struct))))))

(event `EnhancedInput|/Game/Inputs/Action/IA_Move`
  (params (ActionValue :type "Vector2D Structure") (ElapsedSeconds :type "Float (double-precision)") (TriggeredSeconds :type "Float (double-precision)") (InputAction :type "InputAction Object Reference" :default "/Game/Inputs/Action/IA_Move.IA_Move"))
  (:`Triggered`
    (`self.UpdateAnimation` ActionValue ActionValue))
  (:`Canceled`
    (`self.UpdateAnimation` (0.0 0.0) (0.0 0.0) true :!label _label))
  (:`Completed`
    (goto _label)))

(event `EnhancedInput|/Game/Inputs/Action/IA_Interact`
  (params (ActionValue :type Boolean) (ElapsedSeconds :type "Float (double-precision)") (TriggeredSeconds :type "Float (double-precision)") (InputAction :type "InputAction Object Reference" :default "/Game/Inputs/Action/IA_Interact.IA_Interact"))
  (:`Started`
    (for _array_element (`PrimitiveComponent.GetOverlappingActors` (`self.InteractCheck`) null)
      (bind _issuccess (`self.PickUpItem` _array_element))
      (if _issuccess
        (break)
        (else
          (bind _asbp_green (cast `/Game/Blueprint/Character/Green/BP_Green` _array_element))
          (bind _dilogueline (`/Game/Blueprint/Character/Green/BP_Green.GetDialogueLine` _asbp_green))
          (`/Game/Widgets/WBP_MainHUD.SetDialogueLine` (`self.MainHUD`) _dilogueline)
          (break))))
    (`KismetSystemLibrary.RetriggerableDelay` (`self.HideMessageDelay`))
    (`/Game/Widgets/WBP_MainHUD.HideMessageBox` (`self.MainHUD`))))

(fn `PickUpItem`
  (params (Object :type "Object Object Reference"))
  (returns (IsSuccess :type Boolean))
  (bind _asbp_pick_up (cast `/Game/Blueprint/Items/BP_PickUp` Object)
    (:`then`
      (bind (_itemname _itemid) (`/Game/Blueprint/Items/BP_PickUp.GetPickUp` _asbp_pick_up))
      (`/Game/Widgets/WBP_MainHUD.SetItemText` (`self.MainHUD`) _itemname _itemid)
      (return true))
    (:`CastFailed`
      (return false))))

(fn `UpdateAnimation`
  (params (Directionality :type "Vector2D Structure") (InVec :type "Vector2D Structure") (TransitionToIdle :type Boolean))
  (bind (_x _y) (`KismetMathLibrary.BreakVector2D` InVec))
  (bind (_x_2 _y_2) (`KismetMathLibrary.BreakVector2D` InVec))
  (if TransitionToIdle
    (`self.AddMovementInput` (1.0 0.0 0.0) _x)
    (`self.AddMovementInput` (0.0 1.0 0.0) _y)
    (`/Engine/EditorBlueprintResources/StandardMacros.CompareFloat` (`KismetMathLibrary.BreakVector2D` (`self.Directionality`))
      (:`>`
        (`PaperFlipbookComponent.SetFlipbook` (`self.Sprite`) "/Game/PaperAssets/Characters/Red/FB_Red_Idle_R.FB_Red_Idle_R"))
      (:`==`
        (`/Engine/EditorBlueprintResources/StandardMacros.CompareFloat` (`.Y` (`KismetMathLibrary.BreakVector2D` (`self.Directionality`)))
          (:`>`
            (`PaperFlipbookComponent.SetFlipbook` (`self.Sprite`) "/Game/PaperAssets/Characters/Red/FB_Red_Idle_D.FB_Red_Idle_D"))
          (:`<`
            (`PaperFlipbookComponent.SetFlipbook` (`self.Sprite`) "/Game/PaperAssets/Characters/Red/FB_Red_Idle_U.FB_Red_Idle_U"))))
      (:`<`
        (`PaperFlipbookComponent.SetFlipbook` (`self.Sprite`) "/Game/PaperAssets/Characters/Red/FB_Red_Idle_L.FB_Red_Idle_L")))
    (else
      (set `self.Directionality` Directionality)
      (`self.AddMovementInput` (1.0 0.0 0.0) _x_2)
      (`self.AddMovementInput` (0.0 1.0 0.0) _y_2)
      (`/Engine/EditorBlueprintResources/StandardMacros.CompareFloat` (`KismetMathLibrary.BreakVector2D` (`self.Directionality`))
        (:`>`
          (`PaperFlipbookComponent.SetFlipbook` (`self.Sprite`) "/Game/PaperAssets/Characters/Red/FB_Red_Walk_R.FB_Red_Walk_R"))
        (:`==`
          (`/Engine/EditorBlueprintResources/StandardMacros.CompareFloat` (`.Y` (`KismetMathLibrary.BreakVector2D` (`self.Directionality`)))
            (:`>`
              (`PaperFlipbookComponent.SetFlipbook` (`self.Sprite`) "/Game/PaperAssets/Characters/Red/FB_Red_Walk_D.FB_Red_Walk_D"))
            (:`<`
              (`PaperFlipbookComponent.SetFlipbook` (`self.Sprite`) "/Game/PaperAssets/Characters/Red/FB_Red_Walk_U.FB_Red_Walk_U"))))
        (:`<`
          (`PaperFlipbookComponent.SetFlipbook` (`self.Sprite`) "/Game/PaperAssets/Characters/Red/FB_Red_Walk_L.FB_Red_Walk_L"))))))

(fn `UserConstructionScript`)