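; BP_Green is the Blueprint for the Green character, providing lines of dialogue on request.
; GetDialogueLine returns the DialogueLine entry at CurrentIndex and advances the index, wrapping to the first entry once it passes the end, so successive calls cycle through the lines in order.
; The event graph and construction script hold no logic.
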(fn `GetDialogueLine`
  (returns (DilogueLine :type String))
  (locals (LocalDilogueLine :type String))
  (bind _currentindex (`self.CurrentIndex`))
  (if (> (`self.CurrentIndex`) (- (`KismetArrayLibrary.Array_Length` (`self.Dialogue Line`)) 1))
    (set `self.CurrentIndex` 0))
  (bind _output_get (set `local.LocalDilogueLine` (`|GetArrayItem` (`self.Dialogue Line`) _currentindex)))
  (`/Engine/EditorBlueprintResources/StandardMacros.IncrementInt` _currentindex
    (:`  `
      (return _output_get))))

(fn `UserConstructionScript`)